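; BP_Invader_Base is an invader actor, apparently meant as a base class, with a billboard visual and the ability to shoot.
; Its construction script creates a dynamic M_Invader material on the MaterialBillboard and feeds it the actor's icon texture and color.
; The Fire event checks CanFire, then spawns a half-scale BP_Bullet slightly ahead along the actor's forward vector, matching its rotation.
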(event `Fire`
  (bind (_returnvalue_location _returnvalue_rotation) (`KismetMathLibrary.BreakTransform` (`self.GetTransform`)))
  (if (`self.CanFire`)
    (`|SpawnActorFromClass` "/Game/Invader/Blueprints/BP_Bullet.BP_Bullet_C" (`KismetMathLibrary.MakeTransform` (+ _returnvalue_location (* (`self.GetActorForwardVector`) 100.0)) _returnvalue_rotation (0.5 0.5 0.5)) "Undefined" "OverrideRootScale" null null)))

(fn `UserConstructionScript`
  (bind _returnvalue (`PrimitiveComponent.CreateDynamicMaterialInstance` (`self.MaterialBillboard`) 0 "/Game/Invader/Materlas/M_Invader.M_Invader" "None"))
  (bind _output_get (set `self.MaterialInstance` _returnvalue))
  (`MaterialInstanceDynamic.SetTextureParameterValue` _output_get "IconImage" (`self.IconImage_0`))
  (`MaterialInstanceDynamic.SetVectorParameterValue` _output_get "Color" (`self.Color`)))