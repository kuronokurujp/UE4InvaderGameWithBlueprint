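; Space Invaders-style enemy actor that steps sideways and descends when the game mode signals.
; On BeginPlay it binds to BP_GameMode's move and go-down events, shifting a fixed distance along Y or down negative X.
; After each sideways step outside the Y bounds, it messages the game mode that a side was touched and requests the opposite direction.
; Every Tick it polls the game mode for the shared direction.
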(event `self.ReceiveBeginPlay`
  (bind _asbp_game_mode (cast `/Game/Invader/Blueprints/BP_GameMode` (`GameplayStatics.GetGameMode`)))
  (add `/Game/Invader/Blueprints/BP_GameMode.OnMove` _asbp_game_mode (`|CreateDelegate` :!event `OnMove`))
  (add `/Game/Invader/Blueprints/BP_GameMode.OnGoDown` _asbp_game_mode (`|CreateDelegate` :!event `OnGoDown`)))

(event `OnMove`
  (bind (_returnvalue_x _returnvalue_y) (`KismetMathLibrary.BreakVector` (`self.K2_GetActorLocation`)))
  (bind (_returnvalue_x_2 _returnvalue_y_2) (`KismetMathLibrary.BreakVector` (`self.K2_GetActorLocation`)))
  (`self.K2_SetActorLocation` (+ (`self.K2_GetActorLocation`) (`KismetMathLibrary.MakeVector` 0.0 (* (`self.Direction`) 50.0))))
  (`|ExecutionSequence`
    (:`then_0`
      (if (not (`KismetMathLibrary.InRange_FloatFloat` _returnvalue_y_2 -1500.0 1500.0))
        (message `/Game/Invader/Blueprints/BPI_GameMode.TouchSide` (`GameplayStatics.GetGameMode`))
        (if (> _returnvalue_y 0.0)
          (message `/Game/Invader/Blueprints/BPI_GameMode.ReverseDirection` (`GameplayStatics.GetGameMode`) -1)
          (elif (< _returnvalue_y 0.0)
            (message `/Game/Invader/Blueprints/BPI_GameMode.ReverseDirection` (`GameplayStatics.GetGameMode`) 1)))))))

(event `OnGoDown`
  (`self.K2_SetActorLocation` (+ (`self.K2_GetActorLocation`) (-50.0 0.0 0.0))))

(event `self.ReceiveTick`
  (params (DeltaSeconds :type "Float (single-precision)"))
  (bind _direction (message `/Game/Invader/Blueprints/BPI_GameMode.GetDirection` (`GameplayStatics.GetGameMode`)))
  (set `self.Direction` _direction))

(fn `UserConstructionScript`
  (`parent.UserConstructionScript`))