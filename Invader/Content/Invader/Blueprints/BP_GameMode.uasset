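; Game mode for an Invader game that coordinates movement through shared direction and event dispatchers.
; BeginPlay starts a looping timer, and the Move event plays a movement sound, cycling its SoundNumber parameter, then broadcasts OnMove.
; TouchSide broadcasts OnGoDown, while ReverseDirection stores the supplied Direction for retrieval through GetDirection.
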(event `self.ReceiveBeginPlay`
  (`KismetSystemLibrary.K2_SetTimerDelegate` (`|CreateDelegate` :!event `Move`) 1.0 true))

(event `Move`
  (bind _returnvalue (`GameplayStatics.SpawnSound2D` "/Game/Invader/Sounds/S_MovementSound.S_MovementSound" 1.0 1.0 0.0 null))
  (`AudioComponent.SetIntParameter` _returnvalue "SoundNumber" (`self.SoundNumber`))
  (bind _result (`/Engine/EditorBlueprintResources/StandardMacros.IncrementInt` (`self.SoundNumber`))
    (:`  `
      (set `self.SoundNumber` (`KismetMathLibrary.SelectInt` 0 _result (> _result 3)))
      (`self.OnMove`))))

(event `/Game/Invader/Blueprints/BPI_GameMode.TouchSide`
  (`self.OnGoDown`))

(event `/Game/Invader/Blueprints/BPI_GameMode.ReverseDirection`
  (params (Direction :type Integer))
  (set `self.Direction` Direction))

(fn `GetDirection`
  (returns (Direction :type Integer))
  (return (`self.Direction`)))

(fn `UserConstructionScript`)